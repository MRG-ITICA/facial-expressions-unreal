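; Actor component that distributes twist across helper joints along bone segments of the owner's OculusXR body-tracking skeleton.
; Initialize caches each joint's relative spacing and up axis in end-bone space, or destroys the component without body tracking.
; ApplyTwist re-spaces joints along each segment, then blends their rotation from the parent bone's toward a segment-aligned look-at following the end bone's up, by joint and segment weights.
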(event Custom|ApplyTwist
  (for _index (range 0 (- (Utilities|Array|Length (Variables|Default|GetBoneTwistInfos)) 1))
    (CallFunction|SpaceJoints (Utilities|Array|Get(acopy) (Variables|Default|GetBoneTwistInfos) _index))
    (CallFunction|TwistJoints (Utilities|Array|Get(acopy) (Variables|Default|GetBoneTwistInfos) _index))))

(event Custom|Initialize
  (bind _returnvalue (Components|GetOwner))
  (bind _returnvalue_2 (Actor|GetComponentbyClass _returnvalue "/Script/OculusXRMovement.OculusXRBodyTrackingComponent"))
  (Utilities|IsValid _returnvalue_2
    (:Is%20Valid
      (Variables|Default|SetOculusBodyTracking _returnvalue_2)
      (for _index (range 0 (- (Utilities|Array|Length (Variables|Default|GetBoneTwistInfos)) 1))
        (CallFunction|InitializeBoneTwistInfo (Utilities|Array|Get(acopy) (Variables|Default|GetBoneTwistInfos) _index))))
    (:Is%20Not%20Valid
      (Components|DestroyComponent))))

(fn InitializeBoneTwistInfo
  (params (BoneTwistInfo :type F%20Bone%20Twist%20Info%20Structure%20%28by%20ref%29))
  (bind (_segmentend _segmentendup _currentendup) (Utilities|Struct|BreakF_BoneTwistInfo BoneTwistInfo))
  (bind _twistjoints (Utilities|Struct|BreakF_BoneTwistInfo BoneTwistInfo))
  (bind (_twistupaxis _currentendup_2) (Utilities|Struct|BreakF_BoneTwistInfo BoneTwistInfo))
  (bind (_segmentstart _segmentend_2) (Utilities|Struct|BreakF_BoneTwistInfo BoneTwistInfo))
  (bind (_twistforwardaxis _twistupaxis_2 _twistlocalrotationaxisoffset) (Utilities|Struct|BreakF_BoneTwistInfo BoneTwistInfo))
  (|SetBy-RefVar _currentendup (select (!= _segmentendup "") _segmentendup _segmentend))
  (for _index (range 0 (- (Utilities|Array|Length _twistjoints) 1))
    (Utilities|FlowControl|Sequence
      (:then_0
        (bind _returnvalue (Class|PoseableMeshComponent|GetBoneLocationbyName (Variables|Default|GetOculusBodyTracking) (.Joint (Utilities|Struct|BreakF_TwistJoint (Utilities|Array|Get(acopy) _twistjoints _index))) "WorldSpace"))
        (bind _returnvalue_2 (Class|PoseableMeshComponent|GetBoneLocationbyName (Variables|Default|GetOculusBodyTracking) _segmentstart "WorldSpace"))
        (bind _returnvalue_3 (Class|PoseableMeshComponent|GetBoneLocationbyName (Variables|Default|GetOculusBodyTracking) _segmentend_2 "WorldSpace"))
        (Utilities|Array|Add (Utilities|Struct|BreakF_BoneTwistInfo BoneTwistInfo) (/ (Math|Vector|VectorLength (- _returnvalue_3 _returnvalue)) (Math|Vector|VectorLength (- _returnvalue_3 _returnvalue_2)))))
      (:then_1
        (bind _returnvalue_4 (Class|PoseableMeshComponent|GetBoneTransformbyName (Variables|Default|GetOculusBodyTracking) (.Joint (Utilities|Struct|BreakF_TwistJoint (Utilities|Array|Get(acopy) _twistjoints _index))) "ComponentSpace"))
        (bind _returnvalue_5 (Class|PoseableMeshComponent|GetBoneTransformbyName (Variables|Default|GetOculusBodyTracking) _currentendup_2 "ComponentSpace"))
        (|SetBy-RefVar (.SegmentEndUpAxis (Utilities|Struct|BreakF_TwistJoint (Utilities|Array|Get(acopy) _twistjoints _index))) (Math|Transform|InverseTransformDirection _returnvalue_5 (Math|Transform|TransformDirection _returnvalue_4 _twistupaxis))))))
  (|SetBy-RefVar _twistlocalrotationaxisoffset (Class|KismetMathLibrary|NegateRotator (Math|Rotator|MakeRotfromXZ _twistforwardaxis _twistupaxis_2))))

(fn SpaceJoints
  (params (BoneTwistInfo :type F%20Bone%20Twist%20Info%20Structure%20%28by%20ref%29))
  (bind (_segmentstart _segmentend _twistjoints _spacings) (Utilities|Struct|BreakF_BoneTwistInfo BoneTwistInfo))
  (for _index (range 0 (- (Utilities|Array|Length (Utilities|Struct|BreakF_BoneTwistInfo BoneTwistInfo)) 1))
    (bind _returnvalue (Class|PoseableMeshComponent|GetBoneLocationbyName (Variables|Default|GetOculusBodyTracking) _segmentstart "WorldSpace"))
    (bind _returnvalue_2 (Class|PoseableMeshComponent|GetBoneLocationbyName (Variables|Default|GetOculusBodyTracking) _segmentend "WorldSpace"))
    (Class|PoseableMeshComponent|SetBoneLocationbyName (Variables|Default|GetOculusBodyTracking) (Utilities|Struct|BreakF_TwistJoint (Utilities|Array|Get(acopy) _twistjoints _index)) (+ _returnvalue (* (- _returnvalue_2 _returnvalue) (- 1.0 (Utilities|Array|Get(acopy) _spacings _index)))) "WorldSpace")))

(fn TwistJoints
  (params (BoneTwistInfo :type F%20Bone%20Twist%20Info%20Structure%20%28by%20ref%29))
  (bind _twistjoints (Utilities|Struct|BreakF_BoneTwistInfo BoneTwistInfo))
  (bind _oculusbodytracking (Variables|Default|GetOculusBodyTracking))
  (bind (_segmentstart _segmentend _currentlookatdir) (Utilities|Struct|BreakF_BoneTwistInfo BoneTwistInfo))
  (bind (_twistlocalrotationaxisoffset _currentlookatdir_2) (Utilities|Struct|BreakF_BoneTwistInfo BoneTwistInfo))
  (Utilities|FlowControl|Sequence
    (:then_0
      (bind _returnvalue (Class|PoseableMeshComponent|GetBoneLocationbyName (Variables|Default|GetOculusBodyTracking) _segmentstart "ComponentSpace"))
      (bind _returnvalue_2 (Class|PoseableMeshComponent|GetBoneLocationbyName (Variables|Default|GetOculusBodyTracking) _segmentend "ComponentSpace"))
      (|SetBy-RefVar _currentlookatdir (* (- _returnvalue_2 _returnvalue) 2.0)))
    (:then_1
      (for _index (range 0 (- (Utilities|Array|Length _twistjoints) 1))
        (bind _returnvalue_3 (Class|PoseableMeshComponent|GetBoneTransformbyName (Variables|Default|GetOculusBodyTracking) (Utilities|Struct|BreakF_BoneTwistInfo BoneTwistInfo) "ComponentSpace"))
        (bind _returnvalue_4 (Class|PoseableMeshComponent|GetBoneRotationbyName _oculusbodytracking (Class|SkinnedMeshComponent|GetParentBone _oculusbodytracking (.Joint (Utilities|Struct|BreakF_TwistJoint (Utilities|Array|Get(acopy) _twistjoints _index)))) "ComponentSpace"))
        (Components|PoseableMesh|SetBoneRotationbyName (Variables|Default|GetOculusBodyTracking) (.Joint (Utilities|Struct|BreakF_TwistJoint (Utilities|Array|Get(acopy) _twistjoints _index))) (Math|Rotator|Lerp(Rotator) _returnvalue_4 (Math|Rotator|CombineRotators _twistlocalrotationaxisoffset (Math|Rotator|MakeRotfromXZ _currentlookatdir_2 (Math|Transform|TransformDirection _returnvalue_3 (.SegmentEndUpAxis (Utilities|Struct|BreakF_TwistJoint (Utilities|Array|Get(acopy) _twistjoints _index)))))) (* (.Weight (Utilities|Struct|BreakF_TwistJoint (Utilities|Array|Get(acopy) _twistjoints _index))) (Utilities|Struct|BreakF_BoneTwistInfo BoneTwistInfo)) true) "ComponentSpace")))))