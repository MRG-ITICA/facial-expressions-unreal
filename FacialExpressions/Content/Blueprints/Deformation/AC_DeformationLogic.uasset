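; Actor component that deforms Oculus XR body-tracking poses so the skeleton keeps the proportions captured at initialization.
; Initialize records bone lengths along hips-to-head, chest-to-shoulder and shoulder-to-upper-arm, plus hip-to-head distance, destroying itself without tracking.
; ApplyDeformation refreshes bone directions, optionally offsets the spine by the length error, then FixArms restores segment lengths.
; Upper arms can interpolate with threshold snapping, and lower arms follow by weighted offsets.
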(event Custom|Initialize
  (bind _returnvalue (Components|GetOwner))
  (bind _returnvalue_2 (Actor|GetComponentbyClass _returnvalue "/Script/OculusXRMovement.OculusXRBodyTrackingComponent"))
  (Utilities|IsValid _returnvalue_2
    (:Is%20Valid
      (Variables|Default|SetOculusXRBodyTracking _returnvalue_2)
      (Utilities|FlowControl|Sequence
        (:then_0
          ;[1 1 1] Set Hip to Head bone names
          (bind _keys (Utilities|Map|Keys (Variables|/Script/OculusXRMovement.OculusXRBodyTrackingComponent|GetBoneNames (Variables|Default|GetOculusXRBodyTracking))))
          (bind _array_element (Utilities|Array|ForEachLoopwithBreak _keys :!label _label)
            (:LoopBody
              (if (<= (Math|Conversions|ToInteger(Byte) _array_element) (Math|Conversions|ToInteger(Byte) (Utilities|Enum|LiteralenumEOculusXRBoneID "BodyHead")))
                (if (>= (Math|Conversions|ToInteger(Byte) _array_element) (Math|Conversions|ToInteger(Byte) (Utilities|Enum|LiteralenumEOculusXRBoneID "BodyHips")))
                  (if (.ReturnValue (Utilities|Map|Find (Variables|/Script/OculusXRMovement.OculusXRBodyTrackingComponent|GetBoneNames (Variables|Default|GetOculusXRBodyTracking)) _array_element))
                    (Utilities|Array|AddUnique (Variables|Default|GetHipToHeadBoneNames) (.Value (Utilities|Map|Find (Variables|/Script/OculusXRMovement.OculusXRBodyTrackingComponent|GetBoneNames (Variables|Default|GetOculusXRBodyTracking)) _array_element)))))
                (else
                  (goto _label Break))))))
        (:then_1
          (bind _returnvalue_3 (Class|PoseableMeshComponent|GetBoneLocationbyName (Variables|Default|GetOculusXRBodyTracking) "Hips" "ComponentSpace"))
          (bind _returnvalue_4 (Class|PoseableMeshComponent|GetBoneLocationbyName (Variables|Default|GetOculusXRBodyTracking) "Head" "ComponentSpace"))
          (Variables|Default|SetHipToHeadDistance (Math|Vector|Distance(Vector) _returnvalue_4 _returnvalue_3)))
        (:then_2
          (CallFunction|InitializeBonesArray))))
    (:Is%20Not%20Valid
      (Components|DestroyComponent))))

(event Custom|ApplyDeformation
  (for _index (range 0 (- (Utilities|Array|Length (Variables|Default|GetBones)) 1))
    (CallFunction|UpdateDirection (Utilities|Array|Get(acopy) (Variables|Default|GetBones) _index)))
  (if (Utilities|Enum|NotEqual(Enum) (Variables|Default|GetSpineTranslationCorrectionType) "NewEnumerator0")
    (CallFunction|SpineTranslationCorrection))
  (if (Variables|Default|GetFixArms?)
    (CallFunction|FixArms)))

(fn InitializeBonesArray
  (bind _oculusxrbodytracking (Variables|Default|GetOculusXRBodyTracking))
  (bind _leftarmpositioninfo (Variables|Default|GetLeftArmPositionInfo))
  (bind _rightarmpositioninfo (Variables|Default|GetRightArmPositionInfo))
  (bind _hiptoheadbonenames (Variables|Default|GetHipToHeadBoneNames))
  (bind (_shoulderbonename _upperarmbonename) (Utilities|Struct|BreakF_ArmPositionInfo _rightarmpositioninfo))
  (bind (_shoulderbonename_2 _upperarmbonename_2) (Utilities|Struct|BreakF_ArmPositionInfo _leftarmpositioninfo))
  (bind _bonenames (Variables|/Script/OculusXRMovement.OculusXRBodyTrackingComponent|GetBoneNames _oculusxrbodytracking))
  (bind _value (Utilities|Map|Find _bonenames "BodyChest"))
  (Utilities|FlowControl|Sequence
    (:then_0
      (for (_array_element _array_index) _hiptoheadbonenames
        (if (!= (Utilities|Array|LastIndex _hiptoheadbonenames) _array_index)
          (Utilities|Array|Add (Variables|Default|GetBones) (Utilities|Struct|MakeF_BoneDistanceInfo _array_element (Utilities|Array|Get(acopy) _hiptoheadbonenames (+ _array_index 1)))))))
    (:then_1
      (Utilities|Array|Add (Variables|Default|GetBones) (Utilities|Struct|MakeF_BoneDistanceInfo _value (Utilities|Struct|BreakF_ArmPositionInfo (Variables|Default|GetLeftArmPositionInfo))))
      (Utilities|Array|Add (Variables|Default|GetBones) (Utilities|Struct|MakeF_BoneDistanceInfo _value (Utilities|Struct|BreakF_ArmPositionInfo (Variables|Default|GetRightArmPositionInfo)))))
    (:then_2
      (Utilities|Array|Add (Variables|Default|GetBones) (Utilities|Struct|MakeF_BoneDistanceInfo _shoulderbonename_2 _upperarmbonename_2))
      (Utilities|Array|Add (Variables|Default|GetBones) (Utilities|Struct|MakeF_BoneDistanceInfo _shoulderbonename _upperarmbonename)))
    (:then_3
      (for _index (range 0 (- (Utilities|Array|Length (Variables|Default|GetBones)) 1))
        (CallFunction|UpdateDistance (Utilities|Array|Get(acopy) (Variables|Default|GetBones) _index))))))

(fn FixArms
  (bind _rightarmpositioninfo (Variables|Default|GetRightArmPositionInfo))
  (bind _leftarmpositioninfo (Variables|Default|GetLeftArmPositionInfo))
  (bind _leftarmpositioninfo_2 (Variables|Default|GetLeftArmPositionInfo))
  (bind _rightarmpositioninfo_2 (Variables|Default|GetRightArmPositionInfo))
  (bind _rightarmpositioninfo_3 (Variables|Default|GetRightArmPositionInfo))
  (bind _leftarmpositioninfo_3 (Variables|Default|GetLeftArmPositionInfo))
  (bind _rightarmpositioninfo_4 (Variables|Default|GetRightArmPositionInfo))
  (bind _leftarmpositioninfo_4 (Variables|Default|GetLeftArmPositionInfo))
  (bind (_upperarmbonename _upperarmpos) (Utilities|Struct|BreakF_ArmPositionInfo _leftarmpositioninfo_3))
  (bind (_upperarmbonename_2 _movespeed) (Utilities|Struct|BreakF_ArmPositionInfo _rightarmpositioninfo_4))
  (bind (_upperarmbonename_3 _movespeed_2) (Utilities|Struct|BreakF_ArmPositionInfo _leftarmpositioninfo_4))
  (bind (_upperarmbonename_4 _weight _upperarmpos_2) (Utilities|Struct|BreakF_ArmPositionInfo _rightarmpositioninfo_2))
  (bind _lowerarmbonename (Utilities|Struct|BreakF_ArmPositionInfo _rightarmpositioninfo_3))
  (bind (_upperarmbonename_5 _weight_2 _upperarmpos_3) (Utilities|Struct|BreakF_ArmPositionInfo _leftarmpositioninfo))
  (bind _lowerarmbonename_2 (Utilities|Struct|BreakF_ArmPositionInfo _leftarmpositioninfo_2))
  (bind (_upperarmbonename_6 _upperarmpos_4) (Utilities|Struct|BreakF_ArmPositionInfo _rightarmpositioninfo))
  (Utilities|FlowControl|Sequence
    (:then_0
      (bind _returnvalue (Class|PoseableMeshComponent|GetBoneLocationbyName (Variables|Default|GetOculusXRBodyTracking) _upperarmbonename "ComponentSpace"))
      (|SetBy-RefVar _upperarmpos _returnvalue)
      (bind _returnvalue_2 (Class|PoseableMeshComponent|GetBoneLocationbyName (Variables|Default|GetOculusXRBodyTracking) _upperarmbonename_6 "ComponentSpace"))
      (|SetBy-RefVar _upperarmpos_4 _returnvalue_2))
    (:then_1
      (for _index (range 0 (- (Utilities|Array|Length (Variables|Default|GetBones)) 1))
        (if (== (Utilities|Struct|BreakF_BoneDistanceInfo (Utilities|Array|Get(acopy) (Variables|Default|GetBones) _index)) _upperarmbonename_3)
          (CallFunction|UpdateBonePosition (Utilities|Array|Get(acopy) (Variables|Default|GetBones) _index) (Variables|Default|GetMoveTowardsArms) _movespeed_2)
          (elif (Utilities|Name|Equal(Name) (Utilities|Struct|BreakF_BoneDistanceInfo (Utilities|Array|Get(acopy) (Variables|Default|GetBones) _index)) _upperarmbonename_2)
            (CallFunction|UpdateBonePosition (Utilities|Array|Get(acopy) (Variables|Default|GetBones) _index) (Variables|Default|GetMoveTowardsArms) _movespeed)
            (else
              (CallFunction|UpdateBonePosition (Utilities|Array|Get(acopy) (Variables|Default|GetBones) _index) false 1.0))))))
    (:then_2
      (bind _returnvalue_3 (Class|PoseableMeshComponent|GetBoneLocationbyName (Variables|Default|GetOculusXRBodyTracking) _upperarmbonename_5 "ComponentSpace"))
      (bind _returnvalue_4 (Class|PoseableMeshComponent|GetBoneLocationbyName (Variables|Default|GetOculusXRBodyTracking) _lowerarmbonename_2 "ComponentSpace"))
      (Class|PoseableMeshComponent|SetBoneLocationbyName (Variables|Default|GetOculusXRBodyTracking) _lowerarmbonename_2 (+ _returnvalue_4 (* (- _returnvalue_3 _upperarmpos_3) _weight_2)) "ComponentSpace"))
    (:then_3
      (bind _returnvalue_5 (Class|PoseableMeshComponent|GetBoneLocationbyName (Variables|Default|GetOculusXRBodyTracking) _upperarmbonename_4 "ComponentSpace"))
      (bind _returnvalue_6 (Class|PoseableMeshComponent|GetBoneLocationbyName (Variables|Default|GetOculusXRBodyTracking) _lowerarmbonename "ComponentSpace"))
      (Class|PoseableMeshComponent|SetBoneLocationbyName (Variables|Default|GetOculusXRBodyTracking) _lowerarmbonename (+ _returnvalue_6 (* (- _returnvalue_5 _upperarmpos_2) _weight)) "ComponentSpace"))))

(fn UpdateDistance
  (params (BoneDistanceInfo :type F%20Bone%20Distance%20Info%20Structure%20%28by%20ref%29))
  (bind (_startbonename _endbonename _distance) (Utilities|Struct|BreakF_BoneDistanceInfo BoneDistanceInfo))
  (bind _returnvalue (Class|PoseableMeshComponent|GetBoneLocationbyName (Variables|Default|GetOculusXRBodyTracking) _startbonename "ComponentSpace"))
  (bind _returnvalue_2 (Class|PoseableMeshComponent|GetBoneLocationbyName (Variables|Default|GetOculusXRBodyTracking) _endbonename "ComponentSpace"))
  (|SetBy-RefVar _distance (Math|Vector|Distance(Vector) _returnvalue_2 _returnvalue)))

(fn UpdateDirection
  (params (BoneDistanceInfo :type F%20Bone%20Distance%20Info%20Structure%20%28by%20ref%29))
  (bind (_startbonename _endbonename _direction) (Utilities|Struct|BreakF_BoneDistanceInfo BoneDistanceInfo))
  (bind _returnvalue (Class|PoseableMeshComponent|GetBoneLocationbyName (Variables|Default|GetOculusXRBodyTracking) _startbonename "ComponentSpace"))
  (bind _returnvalue_2 (Class|PoseableMeshComponent|GetBoneLocationbyName (Variables|Default|GetOculusXRBodyTracking) _endbonename "ComponentSpace"))
  (|SetBy-RefVar _direction (Math|Vector|Normalize (- _returnvalue_2 _returnvalue))))

(fn UpdateBonePosition
  (params (BoneDistanceInfo :type F%20Bone%20Distance%20Info%20Structure%20%28by%20ref%29) (UseMoveTowards :type Boolean) (MoveSpeed :type Float%20%28double-precision%29))
  (bind (_targetpos _currentpos) (Utilities|Struct|BreakF_BoneDistanceInfo BoneDistanceInfo))
  (bind (_endbonename _currentpos_2) (Utilities|Struct|BreakF_BoneDistanceInfo BoneDistanceInfo))
  (bind (_endbonename_2 _snapthreshold _currentpos_3) (Utilities|Struct|BreakF_BoneDistanceInfo BoneDistanceInfo))
  (bind (_distance _direction _targetpos_2) (Utilities|Struct|BreakF_BoneDistanceInfo BoneDistanceInfo))
  (Utilities|FlowControl|Sequence
    (:then_0
      (bind _returnvalue (Class|PoseableMeshComponent|GetBoneLocationbyName (Variables|Default|GetOculusXRBodyTracking) (Utilities|Struct|BreakF_BoneDistanceInfo BoneDistanceInfo) "ComponentSpace"))
      (|SetBy-RefVar _targetpos_2 (+ _returnvalue (* _direction _distance))))
    (:then_1
      (bind _returnvalue_2 (Class|PoseableMeshComponent|GetBoneLocationbyName (Variables|Default|GetOculusXRBodyTracking) _endbonename_2 "ComponentSpace"))
      (if (>= (Math|Vector|Distance(Vector) _returnvalue_2 _currentpos_3) _snapthreshold)
        (|SetBy-RefVar (Utilities|Struct|BreakF_BoneDistanceInfo BoneDistanceInfo) _returnvalue_2)))
    (:then_2
      (|SetBy-RefVar _currentpos (select UseMoveTowards (Math|Interpolation|VInterpTo _currentpos _targetpos (Utilities|Time|GetWorldDeltaSeconds) MoveSpeed) _targetpos)))
    (:then_3
      (Class|PoseableMeshComponent|SetBoneLocationbyName (Variables|Default|GetOculusXRBodyTracking) _endbonename _currentpos_2 "ComponentSpace"))))

(fn SpineTranslationCorrection
  (bind _oculusxrbodytracking (Variables|Default|GetOculusXRBodyTracking))
  (bind _spinetranslationcorrectiontype (Variables|Default|GetSpineTranslationCorrectionType))
  (bind _oculusxrbodytracking_2 (Variables|Default|GetOculusXRBodyTracking))
  (bind _returnvalue (Class|PoseableMeshComponent|GetBoneLocationbyName _oculusxrbodytracking "Head" "ComponentSpace"))
  (bind _returnvalue_2 (Class|PoseableMeshComponent|GetBoneLocationbyName _oculusxrbodytracking "Hips" "ComponentSpace"))
  (LocalVariables|SetOffset (* (Math|Vector|Normalize (- _returnvalue_2 _returnvalue)) (- (Variables|Default|GetHipToHeadDistance) (Math|Vector|VectorLength (- _returnvalue_2 _returnvalue)))))
  (for _array_element (Variables|Default|GetHipToHeadBoneNames)
    (if (not (Math|Boolean|ORBoolean (and (Utilities|Name|Equal(Name) _array_element "Head") (Utilities|Enum|Equal(Enum) _spinetranslationcorrectiontype "NewEnumerator1")) (and (Utilities|Name|Equal(Name) _array_element "Hips") (Utilities|Enum|Equal(Enum) _spinetranslationcorrectiontype "NewEnumerator2")) (and (Utilities|Enum|Equal(Enum) _spinetranslationcorrectiontype "NewEnumerator3") (or (Utilities|Name|Equal(Name) _array_element "Head") (Utilities|Name|Equal(Name) _array_element "Hips")))))
      (bind _returnvalue_3 (Class|PoseableMeshComponent|GetBoneLocationbyName _oculusxrbodytracking_2 _array_element "ComponentSpace"))
      (Class|PoseableMeshComponent|SetBoneLocationbyName _oculusxrbodytracking_2 _array_element (+ _returnvalue_3 (LocalVariables|GetOffset)) "ComponentSpace"))))